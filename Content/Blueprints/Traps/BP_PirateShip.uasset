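; BP_PirateShip is a pirate ship trap that fires two cannonballs once, when play begins.
; BeginPlay spawns a BP_CannonBall at the transform of each attack cannon component and launches its Ball with a velocity-change impulse.
; The impulses use fixed world-space vectors: LeftAttackSide flips the Y direction, and the second cannon's shot has a stronger downward push.
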(event EventBeginPlay
  (Utilities|FlowControl|Sequence
    (:then_0
      (bind _returnvalue (Game|SpawnActorfromClass "/Game/Blueprints/Traps/BP_CannonBall.BP_CannonBall_C" (Transformation|GetWorldTransform (Variables|Default|GetAttackCannon1)) "Undefined" "MultiplyWithRoot" 0 0))
      (Physics|AddImpulse (Variables|/Game/Blueprints/Traps/BP_CannonBall.BP_CannonBall_C|GetBall _returnvalue) (select (Variables|Default|GetLeftAttackSide) (Math|Vector|MakeVector 0.0 -5e+02 -2e+03) (Math|Vector|MakeVector 0.0 5e+02 -2e+03)) "None" true))
    (:then_1
      (bind _returnvalue_2 (Game|SpawnActorfromClass "/Game/Blueprints/Traps/BP_CannonBall.BP_CannonBall_C" (Transformation|GetWorldTransform (Variables|Default|GetAttackCannon2)) "Undefined" "MultiplyWithRoot" 0 0))
      (Physics|AddImpulse (Variables|/Game/Blueprints/Traps/BP_CannonBall.BP_CannonBall_C|GetBall _returnvalue_2) (select (Variables|Default|GetLeftAttackSide) (Math|Vector|MakeVector 0.0 -5e+02 -3e+03) (Math|Vector|MakeVector 0.0 5e+02 -3e+03)) "None" true))))

(fn ConstructionScript)