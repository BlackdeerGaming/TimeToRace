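; BPP_RocketMap is a rocket Blueprint that plays a one-shot deploy sequence on BeginPlay, then removes itself.
; It shifts the top blocks apart in X and activates a particle trail after a short delay.
; The DeployTime timeline drives a per-update upward world offset and the trail's Niagara gravity.
; When the timeline finishes, it spawns an actor at the mesh's original location and destroys itself shortly after.
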(event EventBeginPlay
  (bind _l_topblock (Variables|Default|GetL_TopBlock))
  (bind _r_topblock (Variables|Default|GetR_TopBlock))
  (Variables|Default|SetInitial%20Location (Transformation|GetWorldLocation (Variables|Default|GetInstancedStaticMesh)))
  (Utilities|FlowControl|Sequence
    (:then_0
      (Utilities|FlowControl|Delay 2.0)
      (Components|Activation|Activate (Variables|Default|GetP_Trail_Converted) true))
    (:then_1
      (Transformation|SetWorldLocation _l_topblock (+ (Transformation|GetWorldLocation _l_topblock) "-1000.000000,0.000000,0.000000") false false)
      (Transformation|SetWorldLocation _r_topblock (+ (Transformation|GetWorldLocation _r_topblock) "1000.000000,0.000000,0.000000") false false))
    (:then_2
      (bind (_direction _deploytimemovement _deployexplosion) (Timeline|DeployTime PlayFromStart)
        (:Update
          (Transformation|AddActorWorldOffset (Math|Vector|MakeVector 0.0 0.0 (Math|Float|Lerp 0.0 8e+02 _deploytimemovement)))
          (Niagara|SetNiagaraVariable(Vector3) (Variables|Default|GetP_Trail_Converted) "User.Gravity" (Math|Vector|MakeVector 0.0 0.0 (Math|Float|Lerp 0.0 -2.5e+03 _deployexplosion))))
        (:Finished
          (Game|SpawnActorfromClass "BPP_RocketMap_C" (Math|Transform|MakeTransform (Variables|Default|GetInitial%20Location) "0, 0, 0" "1.000000,1.000000,1.000000") "Undefined" "MultiplyWithRoot" 0 0)
          (Utilities|FlowControl|Delay 1.0)
          (Actor|DestroyActor))))))

(fn ConstructionScript)