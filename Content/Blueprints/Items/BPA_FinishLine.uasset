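; Finish line actor that ends the car game when a player vehicle crosses it.
; On collision overlap with a VehicleAdvPawn, it matches the pawn's TeamColor as text against blue, green, orange or red to set a win message for Player1 to Player4.
; It then passes that message to FinishTheGame on the BPGM_CarGame game mode.
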(event OnComponentBeginOverlap(Collision)
  (params (OverlappedComponent :type Primitive%20Component%20Object%20Reference) (OtherActor :type Actor%20Object%20Reference) (OtherComp :type Primitive%20Component%20Object%20Reference) (OtherBodyIndex :type Integer) (bFromSweep :type Boolean) (SweepResult :type Hit%20Result%20Structure%20%28by%20ref%29))
  (bind _asvehicle_adv_pawn (Utilities|Casting|CastToVehicleAdvPawn OtherActor))
  (Utilities|WhoWon? (Utilities|String|ToString(Object) (Variables|/Game/Blueprints/Vehicles/Default/VehicleAdvPawn.VehicleAdvPawn_C|GetTeamColor _asvehicle_adv_pawn)))
  (bind _asbpgm_car_game (Utilities|Casting|CastToBPGM_CarGame (Game|GetGameMode)))
  (Default|FinishtheGame _asbpgm_car_game (Variables|Default|GetWhoWonGame)))

(fn ConstructionScript)