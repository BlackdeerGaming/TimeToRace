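; Road trap that pops up and flings any non-immune VehicleAdvPawn that drives into its box.
; A DoOnce-gated overlap starts the BounceRoad timeline to shift the trap, teleports the car upward, then Fling applies a velocity-change impulse with random sign via RandomValue.
; After a delay the timeline reverses and the gate resets, which happens only on this path, so an immune or non-vehicle overlap leaves the trap disarmed.
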(event OnComponentBeginOverlap(Box)
  (params (OverlappedComponent :type Primitive%20Component%20Object%20Reference) (OtherActor :type Actor%20Object%20Reference) (OtherComp :type Primitive%20Component%20Object%20Reference) (OtherBodyIndex :type Integer) (bFromSweep :type Boolean) (SweepResult :type Hit%20Result%20Structure%20%28by%20ref%29))
  (Utilities|FlowControl|DoOnce false :!label _label
    (:Completed
      (if (!= OtherActor self)
        (bind _asvehicle_adv_pawn (Utilities|Casting|CastToVehicleAdvPawn OtherActor))
        (if (not (Variables|/Game/Blueprints/Vehicles/Default/VehicleAdvPawn.VehicleAdvPawn_C|GetImmune? _asvehicle_adv_pawn))
          (Utilities|FlowControl|Sequence
            (:then_0
              (CallFunction|SmoothRoadMovement))
            (:then_1
              ;[0.15 0.15 0.15 0.5] Set the location of the vehicle
              (Transformation|SetActorLocation _asvehicle_adv_pawn (+ (Transformation|GetActorLocation _asvehicle_adv_pawn) "0.000000,0.000000,212.000000") false true)
              (Utilities|FlowControl|Delay 0.2)
              (CallFunction|Fling _asvehicle_adv_pawn)
              (Utilities|FlowControl|Delay (+ (Components|Timeline|GetTimelineLength (Variables|Default|GetBounceRoad)) 8.0))
              (CallFunction|ReverseSmoothRoadMovement)
              (goto _label Reset))))))))

(event Custom|Smooth%20Road%20Movement
  (bind _returnvalue (Transformation|GetActorLocation))
  ;[0.15 0.15 0.15 0.5] Timeline of Smooth Road Bounce
  (Variables|Default|SetSweep true)
  (Variables|Default|SetOffSet "0.000000,0.000000,12.000000")
  (bind _bouncetrack (Timeline|BounceRoad Play)
    (:Update
      (Transformation|SetActorLocation (Math|Vector|Lerp(Vector) _returnvalue (+ _returnvalue (Variables|Default|GetOffSet)) _bouncetrack) (Variables|Default|GetSweep) false))
    (:Finished
      (Variables|Default|SetOffSet "0.000000,0.000000,-12.000000")
      (Variables|Default|SetSweep false))))

(event Custom|Reverse%20Smooth%20Road%20Movement
  (bind _returnvalue (Transformation|GetActorLocation))
  ;[0.15 0.15 0.15 0.5] Timeline of Smooth Road Bounce
  (bind _bouncetrack (Timeline|BounceRoad Reverse)
    (:Update
      (Transformation|SetActorLocation (Math|Vector|Lerp(Vector) _returnvalue (+ _returnvalue (Variables|Default|GetOffSet)) _bouncetrack) (Variables|Default|GetSweep) false))
    (:Finished
      (Variables|Default|SetOffSet "0.000000,0.000000,-12.000000")
      (Variables|Default|SetSweep false))))

(fn ConstructionScript)

(fn Fling
  (params (WhichCar :type Vehicle%20Adv%20Pawn%20Object%20Reference))
  (bind (_xaxis _yaxis _zaxis) (Utilities|RandomValue))
  (bind _mesh (Variables|/Script/ChaosVehicles.WheeledVehiclePawn|GetMesh WhichCar))
  (if (Math|Random|RandomBool)
    (Physics|AddImpulse _mesh (Math|Vector|MakeVector _xaxis _yaxis _zaxis) "None" true)
    (else
      (Physics|AddImpulse _mesh (Math|Vector|MakeVector (* _xaxis -1.0) (* _yaxis -1.0) (* _zaxis -1.0)) "None" true))))